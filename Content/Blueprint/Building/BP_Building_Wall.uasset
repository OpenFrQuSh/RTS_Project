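; Wall building Blueprint that extends a parent building class with its own durability and damage mitigation.
; InitState sets maximum and current health plus defense power, while the construction script sets a fractional damage reduction.
; Its TakeDamage override scales incoming damage by that reduction before passing it to the parent; DefensePower is not used here.
; A key 1 press also shifts the root component along negative world X without sweeping.
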(event `self.ReceiveTick`
  (params (DeltaSeconds :type "Float (single-precision)"))
  (`parent.ReceiveTick` DeltaSeconds))

(event `Key|One`
  (params (Key :type "Key Structure"))
  (bind _defaultsceneroot (`self.DefaultSceneRoot`))
  (:`Pressed`
    (`SceneComponent.K2_SetWorldLocation` _defaultsceneroot (+ (`SceneComponent.K2_GetComponentLocation` _defaultsceneroot) (-20.0 0.0 0.0)) false false)))

(fn `InitState`
  (bind _output_get (set `self.m_MaxHealth` 1000.0))
  (set `self.m_CurrentHealth` _output_get)
  (set `self.DefensePower` 10.0))

(fn `TakeDamage`
  (params (DamageAmount :type "Float (double-precision)"))
  (`parent.TakeDamage` (* DamageAmount (- 1.0 (`self.DamageReduction`)))))

(fn `UserConstructionScript`
  (`parent.UserConstructionScript`)
  (set `self.DamageReduction` 0.3))