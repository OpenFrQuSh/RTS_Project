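; Defensive building Blueprint that extends a parent building class with damage mitigation.
; Its TakeDamage override subtracts DefensePower from incoming damage, clamps the result at zero and passes it to the parent implementation.
; CompleteConstruction and the construction script only call their parents, and the default event nodes are disabled.
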(fn `CompleteConstruction`
  (`parent.CompleteConstruction`))

(fn `TakeDamage`
  (params (DamageAmount :type "Float (double-precision)"))
  (bind _returnvalue (- DamageAmount (`self.DefensePower`)))
  (if (<= _returnvalue 0.0)
    (`parent.TakeDamage` 0.0)
    (else
      (`parent.TakeDamage` _returnvalue))))

(fn `UserConstructionScript`
  (`parent.UserConstructionScript`))