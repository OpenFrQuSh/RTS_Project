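; Base building actor with a timed construction phase, health and destruction.
; On BeginPlay it starts a looping timer that accumulates and prints progress until construction completes, calls an empty InitState, and enables player input.
; AnyDamage is ignored until construction finishes, then lowers health, updates the WBP_Health widget's ratio, and destroys the widget and actor at zero health.
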(event `self.ReceiveBeginPlay`
  (`self.BeginConstruction`)
  (`self.InitState`)
  (`self.EnableInput` (`GameplayStatics.GetPlayerController` 0)))

(event `self.ReceiveTick`
  (params (DeltaSeconds :type "Float (single-precision)")))

(event `self.ReceiveAnyDamage`
  (params (Damage :type "Float (single-precision)") (DamageType :type "DamageType Object Reference") (InstigatedBy :type "Controller Object Reference") (DamageCauser :type "Actor Object Reference"))
  (if (`self.m_bIsConstructed`)
    (`self.TakeDamage` Damage)
    (`KismetSystemLibrary.PrintText` (`|FormatText` "当前生命值{health}" (`self.m_CurrentHealth`)) true true (struct :`R` 0.122674 :`G` 1.0 :`B` 0.172034 :`A` 1.0) 5.0)
    (`KismetSystemLibrary.PrintText` (`|FormatText` "当前受到伤害{damage}" Damage) true true (struct :`R` 1.0 :`G` 0.035935 :`B` 0.098983 :`A` 1.0) 5.0)
    (`/Engine/EditorBlueprintResources/StandardMacros.IsValid` (`self.Widget`)
      (:`Is Valid`
        (bind _aswbp_health (cast `/Game/Blueprint/Building/WBP_Health` (`WidgetComponent.GetUserWidgetObject` (`self.Widget`))))
        (set `/Game/Blueprint/Building/WBP_Health.Health` (/ (`self.m_CurrentHealth`) (`self.m_MaxHealth`)) _aswbp_health)))
    (else
      (`KismetSystemLibrary.PrintText` "建筑还未建造完成，不受伤害" true true (struct :`R` 0.122674 :`G` 1.0 :`B` 0.172034 :`A` 1.0) 5.0))))

(fn `BeginConstruction`
  (set `self.m_bIsConstructed` false)
  (set `self.m_ConstructionProgress` 0.0)
  (bind _returnvalue (`KismetSystemLibrary.K2_SetTimer` null "UpdateConstruction" 0.5 true))
  (set `self.ConstructTimer` _returnvalue))

(fn `CompleteConstruction`
  (set `self.m_bIsConstructed` true))

(fn `DestroyBuilding`
  (`ActorComponent.K2_DestroyComponent` (`self.Widget`))
  (`self.K2_DestroyActor`))

(fn `InitState`)

(fn `TakeDamage`
  (params (DamageAmount :type "Float (double-precision)"))
  (if (`self.m_bIsConstructed`)
    (bind _output_get (set `self.m_CurrentHealth` (- (`self.m_CurrentHealth`) DamageAmount)))
    (if (<= _output_get 0.0)
      (`self.DestroyBuilding`))
    (else
      (`KismetSystemLibrary.PrintText` "建筑还在建造中" true true (struct :`G` 0.66 :`B` 1.0 :`A` 1.0) 15.0))))

(fn `UpdateConstruction`
  (locals (DeltaTime :type "Float (double-precision)" :default 0.5))
  (set `self.m_ConstructionProgress` (+ (/ (`local.DeltaTime`) (`self.m_InitialConstructionTime`)) (`self.m_ConstructionProgress`)))
  (if (>= (`self.m_ConstructionProgress`) 1.0)
    (`self.CompleteConstruction`)
    (`KismetSystemLibrary.PrintText` (`|FormatText` "建造完成") true true (struct :`G` 0.66 :`B` 1.0 :`A` 1.0) 15.0)
    (`KismetSystemLibrary.K2_ClearAndInvalidateTimerHandle` (`self.ConstructTimer`))
    (else
      (`KismetSystemLibrary.PrintText` (`|FormatText` "当前进度{x}！！" (`self.m_ConstructionProgress`)) true true (struct :`G` 0.66 :`B` 1.0 :`A` 1.0) 15.0))))

(fn `UserConstructionScript`)