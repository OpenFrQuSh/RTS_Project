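; Defensive turret building that automatically aims at and shoots the nearest actor of EnemyType, currently set to BP_Building_Wall, within attack range.
; A looping timer scans the detection sphere for a target, while Tick drops targets that leave range.
; Once constructed, it snaps the turret mesh toward the target and launches an impulse-driven BP_Projectile.
; A fire-rate timer resets the cooldown and re-aims; InitState sets health and combat stats.
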(event `self.ReceiveBeginPlay`
  (`parent.ReceiveBeginPlay`)
  (`KismetSystemLibrary.K2_SetTimer` null "ScanForEnemies" (`self.ScanInterval`) true))

(event `self.ReceiveTick`
  (params (DeltaSeconds :type "Float (single-precision)"))
  (`parent.ReceiveTick` DeltaSeconds)
  (`/Engine/EditorBlueprintResources/StandardMacros.IsValid` (`self.CurrentTarget`)
    (:`Is Valid`
      (if (> (`self.GetDistanceTo` (`self.CurrentTarget`)) (`self.AttackRange`))
        (set `self.CurrentTarget` null)))))

(fn `AimAtTarget`
  (`/Engine/EditorBlueprintResources/StandardMacros.IsValid` (`self.CurrentTarget`)
    (:`Is Valid`
      (`SceneComponent.K2_SetWorldRotation` (`self.TurretMesh`) (`KismetMathLibrary.FindLookAtRotation` (`SceneComponent.K2_GetComponentLocation` (`self.TurretMesh`)) (`self.K2_GetActorLocation` (`self.CurrentTarget`))) false false)
      (if (`self.bCanFire`)
        (`self.FireAtTarget`)))))

(fn `CompleteConstruction`
  (`parent.CompleteConstruction`))

(fn `FireAtTarget`
  (bind (_returnvalue_location _returnvalue_rotation) (`KismetMathLibrary.BreakTransform` (`SceneComponent.K2_GetComponentToWorld` (`self.MuzzlePoint`))))
  (`|ExecutionSequence`
    (:`then_0`
      (set `self.bCanFire` false)
      (bind _returnvalue (`|SpawnActorFromClass` "/Game/Blueprint/Building/BP_Projectile.BP_Projectile_C" (`KismetMathLibrary.MakeTransform` _returnvalue_location _returnvalue_rotation) "Undefined" "MultiplyWithRoot" null null))
      (set `/Game/Blueprint/Building/BP_Projectile.Base Damage` (`self.AttackDamage`) _returnvalue)
      (`PrimitiveComponent.AddVelocityChangeImpulseAtLocation` (`/Game/Blueprint/Building/BP_Projectile.Sphere1` _returnvalue) (* (`self.GetActorForwardVector` _returnvalue) 1000.0) (0.0 0.0 0.0) "None")
      (`self.SetLifeSpan` _returnvalue 10.0))
    (:`then_1`
      (`KismetSystemLibrary.K2_SetTimer` null "ResetFireCooldown" (/ 1.0 (`self.FireRate`))))))

(fn `InitState`
  (bind _output_get (set `self.m_MaxHealth` 1000.0))
  (set `self.m_CurrentHealth` _output_get)
  (set `self.DefensePower` 10.0)
  (set `self.EnemyType` "/Game/Blueprint/Building/BP_Building_Wall.BP_Building_Wall_C")
  (bind _output_get_2 (set `self.AttackRange` 1000.0))
  (`SphereComponent.SetSphereRadius` (`self.DetectionSphereSphere`) _output_get_2 true)
  (set `self.AttackDamage` 100.0)
  (set `self.FireRate` 1.5))

(fn `ResetFireCooldown`
  (set `self.bCanFire` true)
  (`/Engine/EditorBlueprintResources/StandardMacros.IsValid` (`self.CurrentTarget`)
    (:`Is Valid`
      (`self.AimAtTarget`))))

(fn `ScanForEnemies`
  (locals (MinDistance :type "Float (double-precision)") (ClosestEnemy :type "Actor Object Reference"))
  (`|ExecutionSequence`
    (:`then_0`
      (set `local.MinDistance` (`self.AttackRange`))
      (for _array_element (`PrimitiveComponent.GetOverlappingActors` (`self.DetectionSphereSphere`) (`self.EnemyType`))
        (if (`KismetMathLibrary.ClassIsChildOf` (`GameplayStatics.GetObjectClass` _array_element) (`self.EnemyType`))
          (bind _returnvalue (`self.GetDistanceTo` _array_element))
          (if (< _returnvalue (`local.MinDistance`))
            (set `local.ClosestEnemy` _array_element)
            (set `local.MinDistance` _returnvalue)))))
    (:`then_1`
      (`/Engine/EditorBlueprintResources/StandardMacros.IsValid` (`local.ClosestEnemy`)
        (:`Is Valid`
          (set `self.CurrentTarget` (`local.ClosestEnemy`))
          (if (`self.m_bIsConstructed`)
            (`self.AimAtTarget`)
            (else
              (`KismetSystemLibrary.PrintText` "建筑还在建造"))))
        (:`Is Not Valid`
          (set `self.CurrentTarget` null))))))

(fn `StartAttackTimer`)

(fn `UserConstructionScript`
  (`parent.UserConstructionScript`))