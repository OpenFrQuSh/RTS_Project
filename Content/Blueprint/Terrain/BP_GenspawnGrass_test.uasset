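; Test terrain actor that builds a square grid of instanced ground tiles and contains a draft A* pathfinder for that grid.
; The construction script adds 25x25 HISM instances spaced by HexSize, mapping each instance index to its cell data in GridIndex.
; FUNC_FindWayA* searches four-way neighbours using open/closed sets and Manhattan costs from FUNC_Count.
; The search is unfinished: nothing here calls it, it returns no path, and debug prints remain.
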(event `self.ReceiveBeginPlay`
  (`InstancedStaticMeshComponent.SetNumCustomDataFloats` (`self.HISM_Ground1`) 5))

(fn `FUNC_Count`
  (params (Current :type "/Game/Blueprint/Data/GridStatusData Structure") (Gcost :type "/Game/Blueprint/Data/GridStatusData Structure (by ref)") (Hcost :type "/Game/Blueprint/Data/GridStatusData Structure (by ref)"))
  (returns (G :type Integer) (H :type Integer) (F :type Integer))
  (bind (_local_position_x _local_position_y) (break `/Game/Blueprint/Data/GridStatusData` Hcost))
  (bind (_local_position_x_2 _local_position_y_2) (break `/Game/Blueprint/Data/GridStatusData` Gcost))
  (bind (_local_position_x_3 _local_position_y_3) (break `/Game/Blueprint/Data/GridStatusData` Current))
  (bind _returnvalue (+ (`KismetMathLibrary.Abs_Int` (- _local_position_x_3 _local_position_x_2)) (`KismetMathLibrary.Abs_Int` (- _local_position_y_3 _local_position_y_2))))
  (bind _returnvalue_2 (+ (`KismetMathLibrary.Abs_Int` (- _local_position_x_3 _local_position_x)) (`KismetMathLibrary.Abs_Int` (- _local_position_y_3 _local_position_y))))
  (return _returnvalue _returnvalue_2 (+ _returnvalue _returnvalue_2)))

(fn `FUNC_FindWayA*`
  (params (StartPosition :type Integer) (EndPosition :type Integer))
  (locals (Current :type "/Game/Blueprint/Data/Grid_A_FindWay_Data Structure") (OpenList :type "Set of /Game/Blueprint/Data/Grid_A_FindWay_Data Structure") (ClosedList :type "Set of /Game/Blueprint/Data/Grid_A_FindWay_Data Structure") (FourCirculation :type "Array of Vector2D Structure") (MAXf :type Integer :default 99999) (FinishLine :type "/Game/Blueprint/Data/Grid_A_FindWay_Data Structure") (TemporaryStoragePoint :type "/Game/Blueprint/Data/Grid_A_FindWay_Data Structure") (StartLine :type "/Game/Blueprint/Data/Grid_A_FindWay_Data Structure"))
  (bind _gridindex (`self.GridIndex`))
  (bind _temporarystoragepoint (`local.TemporaryStoragePoint`))
  (bind _current_seltgridstatusdata (break `/Game/Blueprint/Data/Grid_A_FindWay_Data` (`local.Current`)))
  (bind (_temporarystoragepoint_seltgridstatusdata _temporarystoragepoint_start_cost _temporarystoragepoint_end_cost _temporarystoragepoint_start_end_cost _temporarystoragepoint_parent _temporarystoragepoint_bisblock) (break `/Game/Blueprint/Data/Grid_A_FindWay_Data` (`local.TemporaryStoragePoint`)))
  (bind _openlist (`local.OpenList`))
  (bind _finishline (`local.FinishLine`))
  (bind _current (`local.Current`))
  (bind _current_2 (`local.Current`))
  (bind (_seltgridstatusdata _start_cost _end_cost _start_end_cost _parent) (break `/Game/Blueprint/Data/Grid_A_FindWay_Data` _temporarystoragepoint))
  (bind _value (`BlueprintMapLibrary.Map_Find` _gridindex EndPosition))
  (bind _value_2 (`BlueprintMapLibrary.Map_Find` _gridindex StartPosition))
  (bind ((`SeltGridStatusData_29_7B7EBD8B47D01B97570CEB859619FE17` _seltgridstatusdata_2)) (break `/Game/Blueprint/Data/Grid_A_FindWay_Data` _value_2))
  (bind (_g _h _f) (`self.FUNC_Count` _seltgridstatusdata (`.SeltGridStatusData_29_7B7EBD8B47D01B97570CEB859619FE17` (break `/Game/Blueprint/Data/Grid_A_FindWay_Data` (`local.Current`))) (`.SeltGridStatusData_29_7B7EBD8B47D01B97570CEB859619FE17` (break `/Game/Blueprint/Data/Grid_A_FindWay_Data` (`local.FinishLine`)))))
  (bind (_g_2 _h_2 _f_2) (`self.FUNC_Count` (`.SeltGridStatusData_29_7B7EBD8B47D01B97570CEB859619FE17` (break `/Game/Blueprint/Data/Grid_A_FindWay_Data` (`local.Current`))) (`.SeltGridStatusData_29_7B7EBD8B47D01B97570CEB859619FE17` (break `/Game/Blueprint/Data/Grid_A_FindWay_Data` _value_2)) (`.SeltGridStatusData_29_7B7EBD8B47D01B97570CEB859619FE17` (break `/Game/Blueprint/Data/Grid_A_FindWay_Data` _value))))
  (`BlueprintSetLibrary.Set_Clear` (`local.ClosedList`))
  (`BlueprintSetLibrary.Set_Clear` (`local.OpenList`))
  (set `local.StartLine` _value_2)
  (set `local.Current` (make `/Game/Blueprint/Data/Grid_A_FindWay_Data` :`SeltGridStatusData` _seltgridstatusdata_2))
  (set `local.FinishLine` _value)
  (bind _output_get (set `local.Current` (make `/Game/Blueprint/Data/Grid_A_FindWay_Data` _seltgridstatusdata_2 _g_2 _h_2 _f_2 _seltgridstatusdata_2)))
  (`BlueprintSetLibrary.Set_Add` _openlist _output_get)
  (while (`BlueprintSetLibrary.Set_IsNotEmpty` _openlist)
    (for _index (range (`BlueprintSetLibrary.Set_Length` _openlist))
      (bind _result (`BlueprintSetLibrary.Set_ToArray` (`local.OpenList`)))
      (`KismetSystemLibrary.PrintString` "asdwasdwd")
      (bind _output (`|GetArrayItem` _result _index))
      (bind ((`Start_End_Cost_17_70C505F14A593B8E78E8C489187EC57A` _start_end_cost_2)) (break `/Game/Blueprint/Data/Grid_A_FindWay_Data` _output))
      (if (< _start_end_cost_2 (`local.MAXf`))
        (set `local.MAXf` _start_end_cost_2)
        (bind _output_get_2 (set `local.Current` _output))
        (if (and (== (break `/Game/Blueprint/Data/GridStatusData` (break `/Game/Blueprint/Data/Grid_A_FindWay_Data` _output_get_2)) (break `/Game/Blueprint/Data/GridStatusData` (break `/Game/Blueprint/Data/Grid_A_FindWay_Data` _finishline))) (== (`.Local_Position_Y_4_FB72CAFC41BC4E66B28491B9444FA8DB` (break `/Game/Blueprint/Data/GridStatusData` (break `/Game/Blueprint/Data/Grid_A_FindWay_Data` _output_get_2))) (`.Local_Position_Y_4_FB72CAFC41BC4E66B28491B9444FA8DB` (break `/Game/Blueprint/Data/GridStatusData` (break `/Game/Blueprint/Data/Grid_A_FindWay_Data` _finishline)))))
          (`BlueprintSetLibrary.Set_Clear` (`local.OpenList`))
          (else
            (`BlueprintSetLibrary.Set_Remove` (`local.OpenList`) _current)
            (`BlueprintSetLibrary.Set_Add` (`local.ClosedList`) _current)
            (for _array_element (`local.FourCirculation`)
              (bind _returnvalue (+ (`KismetMathLibrary.BreakVector2D` _array_element) (break `/Game/Blueprint/Data/GridStatusData` (break `/Game/Blueprint/Data/Grid_A_FindWay_Data` _current_2))))
              (bind _returnvalue_2 (+ (`.Y` (`KismetMathLibrary.BreakVector2D` _array_element)) (`.Local_Position_Y_4_FB72CAFC41BC4E66B28491B9444FA8DB` (break `/Game/Blueprint/Data/GridStatusData` (break `/Game/Blueprint/Data/Grid_A_FindWay_Data` _current_2)))))
              (if (not (or (or (< _returnvalue 0) (>= _returnvalue (`self.Horizontal Axis Quantity`))) (or (< _returnvalue_2 0) (>= _returnvalue_2 (`self.Vertical Axis Quantity`)))))
                (set `local.TemporaryStoragePoint` (make `/Game/Blueprint/Data/Grid_A_FindWay_Data` (make `/Game/Blueprint/Data/GridStatusData` _returnvalue _returnvalue_2) (`.Start_Cost_22_5A28FDED4DE293C5BAA560833CF21C33` (break `/Game/Blueprint/Data/Grid_A_FindWay_Data` _current_2)) (`.End_Cost_21_FD3BAF494C721DB269F315BA5BFEDAA2` (break `/Game/Blueprint/Data/Grid_A_FindWay_Data` _current_2)) (`.Start_End_Cost_17_70C505F14A593B8E78E8C489187EC57A` (break `/Game/Blueprint/Data/Grid_A_FindWay_Data` _current_2)) (`.Parent_24_A2CF78594DBAD44D2CCB3A8C7140AE8C` (break `/Game/Blueprint/Data/Grid_A_FindWay_Data` _current_2)) (`.bisblock_25_DF1705184AA3DD1559D4D79D6E957C1E` (break `/Game/Blueprint/Data/Grid_A_FindWay_Data` _current_2))))
                (if _temporarystoragepoint_bisblock
                  _
                  (elif (`BlueprintSetLibrary.Set_Contains` (`local.ClosedList`) (`local.TemporaryStoragePoint`))
                    _
                    (elif (`BlueprintSetLibrary.Set_Contains` (`local.OpenList`) _temporarystoragepoint)
                      (bind _result_2 (`BlueprintSetLibrary.Set_ToArray` (`local.OpenList`)))
                      (for (_array_element_2 _array_index) _result_2
                        (bind ((`SeltGridStatusData_29_7B7EBD8B47D01B97570CEB859619FE17` _seltgridstatusdata_3) (`Start_Cost_22_5A28FDED4DE293C5BAA560833CF21C33` _start_cost_2) (`End_Cost_21_FD3BAF494C721DB269F315BA5BFEDAA2` _end_cost_2)) (break `/Game/Blueprint/Data/Grid_A_FindWay_Data` _array_element_2))
                        (bind _g_3 (`self.FUNC_Count` _seltgridstatusdata_3 _current_seltgridstatusdata))
                        (if (< _g_3 _start_cost_2)
                          (`KismetArrayLibrary.Array_Set` _result_2 _array_index (make `/Game/Blueprint/Data/Grid_A_FindWay_Data` _seltgridstatusdata_3 _g_3 _end_cost_2 (+ _g_3 _end_cost_2) _current_seltgridstatusdata))))
                      (else
                        (bind _output_get_3 (set `local.TemporaryStoragePoint` (make `/Game/Blueprint/Data/Grid_A_FindWay_Data` _seltgridstatusdata _g _h _f _parent)))
                        (`BlueprintSetLibrary.Set_Add` (`local.OpenList`) _output_get_3)))))))))
        (else
          (`BlueprintSetLibrary.Set_Clear` (`local.OpenList`))
          (`KismetSystemLibrary.PrintString` "Hello"))))))

(fn `FUNC_SpawnTerrain`
  (params (Horizontal_axis_quantity :type Integer) (Vertical_axis_quantity :type Integer))
  (locals (HISM_Size :type Integer :default 100) (HexSize :type "Float (double-precision)" :default 100.0) (world_X :type "Float (double-precision)") (world_y :type "Float (double-precision)") (`index x` :type Integer) (`index y` :type Integer))
  (set `self.Horizontal Axis Quantity` Horizontal_axis_quantity)
  (set `self.Vertical Axis Quantity` Vertical_axis_quantity)
  (for _index (range Horizontal_axis_quantity)
    (set `local.index x` _index)
    (for _index_2 (range Vertical_axis_quantity)
      (set `local.index y` _index_2)
      (set `local.world_X` (* _index (`local.HexSize`) 1.0))
      (set `local.world_y` (* _index_2 (`local.HexSize`) 1.0))
      (bind _returnvalue (`InstancedStaticMeshComponent.AddInstance` (`self.HISM_Ground1`) (`KismetMathLibrary.MakeTransform` (`KismetMathLibrary.MakeVector` (`local.world_X`) (`local.world_y`))) false))
      (`BlueprintMapLibrary.Map_Add` (`self.GridIndex`) _returnvalue (make `/Game/Blueprint/Data/Grid_A_FindWay_Data` (make `/Game/Blueprint/Data/GridStatusData` (`local.index x`) (`local.index y`)))))))

(fn `UserConstructionScript`
  (`self.FUNC_SpawnTerrain` 25 25))