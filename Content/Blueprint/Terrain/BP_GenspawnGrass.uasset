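; Terrain actor that lays out a flat hex-style grid of HISMGround1 instances, apparently grass ground tiles.
; The Construction Script calls FU_SpawnGridMesh, which fills a fixed-size grid in local space, shifting odd rows half a tile.
; FUNC_SpawnTerrain is an unconnected alternative layout whose stagger check can never be true.
; The Event Graph holds only disabled placeholder events, so nothing runs on BeginPlay or Tick.
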(fn `FU_SpawnGridMesh`
  (params (GridWidth :type Integer) (GridHeight :type Integer) (HexFloat :type "Float (double-precision)"))
  (locals (`Local HexWidth` :type "Float (double-precision)") (`Local HexHeight` :type "Float (double-precision)") (`Index y` :type Integer) (`Index x` :type Integer) (x :type Integer) (y :type Integer) (WorldLocation :type "Vector Structure"))
  (bind _local_hexwidth (`local.Local HexWidth`))
  (set `local.Local HexWidth` (* HexFloat 0.7))
  (set `local.Local HexHeight` (* (`KismetMathLibrary.Sqrt` 1.5) HexFloat))
  (for _index (range GridHeight)
    (set `local.Index y` _index)
    (for _index_2 (range GridWidth)
      (set `local.Index x` _index_2)
      (if (== (mod _index 2) 0)
        (set `local.x` (* _index_2 _local_hexwidth))
        (else
          (set `local.x` (+ (* _index_2 _local_hexwidth) (* _local_hexwidth 0.5)))))
      (set `local.y` (* _index (`local.Local HexHeight`) 0.5))
      (bind _output_get (set `local.WorldLocation` (`KismetMathLibrary.MakeVector` (`KismetMathLibrary.Conv_IntToDouble` (`local.x`)) (`KismetMathLibrary.Conv_IntToDouble` (`local.y`)))))
      (`InstancedStaticMeshComponent.AddInstance` (`self.HISM_Ground1`) (`KismetMathLibrary.MakeTransform` _output_get) false))))

(fn `FUNC_SpawnTerrain`
  (params (Horizontal_axis_quantity :type Integer) (Vertical_axis_quantity :type Integer))
  (locals (HISM_Size :type Integer :default 100) (Offset :type "Float (double-precision)") (HexWidth :type "Float (double-precision)") (HexHeight :type "Float (double-precision)") (world_X :type "Float (double-precision)") (world_y :type "Float (double-precision)"))
  (bind _hism_size (`local.HISM_Size`))
  (set `local.HexWidth` (`KismetMathLibrary.Conv_IntToDouble` (* _hism_size 2)))
  (set `local.HexHeight` (`KismetMathLibrary.Conv_IntToDouble` (* _hism_size (`KismetMathLibrary.Sqrt` 1.0))))
  (for _index (range Horizontal_axis_quantity)
    (for _index_2 (range Vertical_axis_quantity)
      (set `local.world_X` (* _index (`local.HexWidth`) 0.55))
      (set `local.world_y` (* _index_2 (`local.HexHeight`)))
      (if (== (`KismetMathLibrary.And_IntInt` _index 2) 1)
        (set `local.world_y` (`KismetMathLibrary.Conv_IntToDouble` (* _index_2 (/ (`local.HexHeight`) 2.0)))))
      (`InstancedStaticMeshComponent.AddInstance` (`self.HISM_Ground1`) (`KismetMathLibrary.MakeTransform` (`KismetMathLibrary.MakeVector` (`local.world_X`) (`local.world_y`))) false))))

(fn `UserConstructionScript`
  (`self.FU_SpawnGridMesh` 50 50 250.0))