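; BP_PlayerPawn is a player pawn driven by Enhanced Input, with planar movement and player-controlled pitch rotation.
; Move input feeds FloatingPawnMovement on X and Y, while rotation input sets RotatingMovement's pitch rate and zeroes it on release or cancel.
; The jump input runs a timeline that eases rotation back to the BeginPlay orientation, blocking new rotation input meanwhile.
; If already near that orientation, jump only prints a debug string.
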(event `self.ReceiveBeginPlay`
  (bind _returnvalue (pcsubsystem `EnhancedInputLocalPlayerSubsystem` (`GameplayStatics.GetPlayerController` 0)))
  (set `self.Initial Rotation` (`self.K2_GetActorRotation`))
  (`/Engine/EditorBlueprintResources/StandardMacros.IsValid` _returnvalue
    (:`Is Valid`
      (`EnhancedInputSubsystemInterface.AddMappingContext` _returnvalue "/Game/Input/BP_PlayerInputMappingContext.BP_PlayerInputMappingContext" 0 (struct)))))

(event `EnhancedInput|/Game/Input/BP_PlayerInputMOVE`
  (params (ActionValue :type "Vector2D Structure") (ElapsedSeconds :type "Float (double-precision)") (TriggeredSeconds :type "Float (double-precision)") (InputAction :type "InputAction Object Reference" :default "/Game/Input/BP_PlayerInputMOVE.BP_PlayerInputMOVE"))
  (bind (_x _y) (`KismetMathLibrary.BreakVector2D` ActionValue))
  (:`Triggered`
    (`PawnMovementComponent.AddInputVector` (`self.FloatingPawnMovement`) (`KismetMathLibrary.MakeVector` _x _y) false)))

(event `EnhancedInput|/Game/Input/BP_PlayerInputRotation`
  (params (ActionValue :type "Float (double-precision)") (ElapsedSeconds :type "Float (double-precision)") (TriggeredSeconds :type "Float (double-precision)") (InputAction :type "InputAction Object Reference" :default "/Game/Input/BP_PlayerInputRotation.BP_PlayerInputRotation"))
  (bind _rotatingmovement (`self.RotatingMovement`))
  (:`Triggered`
    (if (`self.In progress`)
      (set `RotatingMovementComponent.RotationRate` (`KismetMathLibrary.MakeRotator` (.roll (`RotatingMovementComponent.RotationRate` _rotatingmovement)) (* ActionValue (`self.Rotation Speed`)) (.yaw (`RotatingMovementComponent.RotationRate` _rotatingmovement))) _rotatingmovement)))
  (:`Canceled`
    (set `RotatingMovementComponent.RotationRate` (struct) _rotatingmovement :!label _label))
  (:`Completed`
    (goto _label)))

(event `EnhancedInput|/Game/Input/BP_PlayerInputJump`
  (params (ActionValue :type Boolean) (ElapsedSeconds :type "Float (double-precision)") (TriggeredSeconds :type "Float (double-precision)") (InputAction :type "InputAction Object Reference" :default "/Game/Input/BP_PlayerInputJump.BP_PlayerInputJump"))
  (:`Started`
    (if (== (`self.K2_GetActorRotation`) (`self.Initial Rotation`) :`ErrorTolerance` 1.0)
      (`KismetSystemLibrary.PrintString` "Hello" true true (struct :`R` 0.070812 :`G` 0.183171 :`B` 1.0 :`A` 1.0))
      (else
        (set `self.In progress` false)
        (bind (_direction _difference) (`Timeline|Somothly Roate The Initial Position` :!via `PlayFromStart`)
          (:`Update`
            (`self.K2_SetActorRotation` (`KismetMathLibrary.RLerp` (`self.K2_GetActorRotation`) (`self.Initial Rotation`) _difference)))
          (:`Finished`
            (set `self.In progress` true)))))))

(fn `UserConstructionScript`)